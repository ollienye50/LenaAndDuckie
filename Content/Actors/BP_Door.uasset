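; BP_Door is a locked door actor that opens by removing itself when the overlapping actor holds a key.
; On Box overlap it looks for a BPC_KeyPickup component on the other actor and checks its key count.
; With a key it calls the component's Door function and destroys itself; otherwise it prints a hint to go get a key.
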(event `self.Box.OnComponentBeginOverlap`
  (params (OverlappedComponent :type "PrimitiveComponent Object Reference") (OtherActor :type "Actor Object Reference") (OtherComp :type "PrimitiveComponent Object Reference") (OtherBodyIndex :type Integer) (bFromSweep :type Boolean) (SweepResult :type "HitResult Structure (by ref)"))
  (bind _returnvalue (`self.GetComponentByClass` OtherActor "/Game/Actors/BPC_KeyPickup.BPC_KeyPickup_C"))
  (`/Engine/EditorBlueprintResources/StandardMacros.IsValid` _returnvalue
    (:`Is Valid`
      (set `self.KeyGot` _returnvalue)
      (if (> (`/Game/Actors/BPC_KeyPickup.KeyGot` (`self.KeyGot`)) 0)
        (`/Game/Actors/BPC_KeyPickup.Door` (`self.KeyGot`))
        (`self.K2_DestroyActor`)
        (else
          (`KismetSystemLibrary.PrintString` "Go Get Key"))))))

(fn `UserConstructionScript`)