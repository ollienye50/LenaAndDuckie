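; BP_Key is a key pickup actor that is collected by overlapping an actor with a BPC_KeyPickup component.
; If that component's KeyPickedUP flag is true, it calls KeyPickup, plays a sound and destroys itself.
; It then shows a WB_KeyPickup widget, with removal of all widgets queued behind a delay that follows DestroyActor.
; An older player-character check remains unconnected.
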(event `self.Box.OnComponentBeginOverlap`
  (params (OverlappedComponent :type "PrimitiveComponent Object Reference") (OtherActor :type "Actor Object Reference") (OtherComp :type "PrimitiveComponent Object Reference") (OtherBodyIndex :type Integer) (bFromSweep :type Boolean) (SweepResult :type "HitResult Structure (by ref)")))

(event `self.ReceiveActorBeginOverlap`
  (params (OtherActor :type "Actor Object Reference"))
  (bind _returnvalue (`self.GetComponentByClass` OtherActor "/Game/Actors/BPC_KeyPickup.BPC_KeyPickup_C"))
  (bind _keygot (`self.KeyGot`))
  (`/Engine/EditorBlueprintResources/StandardMacros.IsValid` _returnvalue
    (:`Is Valid`
      (set `self.KeyGot` _returnvalue)
      (if (`/Game/Actors/BPC_KeyPickup.KeyPickedUP?` _keygot)
        (`/Game/Actors/BPC_KeyPickup.KeyPickup` _keygot)
        (`GameplayStatics.PlaySound2D` "/Game/Sounds/347172__davidsraba__coin-pickup-sound.347172__davidsraba__coin-pickup-sound" 1.0 1.0 0.0 null null)
        (`KismetSystemLibrary.PrintString` "Key Destroyed")
        (`self.K2_DestroyActor`)
        (bind _returnvalue_2 (`|CreateWidget` "/Game/Levels/Level_1/WB_KeyPickup.WB_KeyPickup_C"))
        (`UserWidget.AddToViewport` _returnvalue_2 0)
        (`KismetSystemLibrary.Delay` 3.0)
        (`WidgetLayoutLibrary.RemoveAllWidgets`)))))

(fn `UserConstructionScript`)