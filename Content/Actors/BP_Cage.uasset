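; BP_Cage is a cage actor that triggers the game's ending sequence when the player pawn overlaps its Box.
; The overlap hides the actor and disables collision on the Box and its cube components.
; Timed Delays then show the WB_Vita1, WB_Vita2 and WB_Lena widgets in turn, clearing all widgets after each, and finally quit the game.
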(event `self.Box.OnComponentBeginOverlap`
  (params (OverlappedComponent :type "PrimitiveComponent Object Reference") (OtherActor :type "Actor Object Reference") (OtherComp :type "PrimitiveComponent Object Reference") (OtherBodyIndex :type Integer) (bFromSweep :type Boolean) (SweepResult :type "HitResult Structure (by ref)"))
  (if (== OtherActor (`GameplayStatics.GetPlayerPawn` 0))
    (`self.SetActorHiddenInGame` true)
    (`PrimitiveComponent.SetCollisionEnabled` (`self.Cube8`) "NoCollision")
    (`PrimitiveComponent.SetCollisionEnabled` (`self.Cube7`) "NoCollision")
    (`PrimitiveComponent.SetCollisionEnabled` (`self.Box`) "NoCollision")
    (`PrimitiveComponent.SetCollisionEnabled` (`self.Cube`) "NoCollision")
    (`PrimitiveComponent.SetCollisionEnabled` (`self.Cube1`) "NoCollision")
    (`PrimitiveComponent.SetCollisionEnabled` (`self.Cube2`) "NoCollision")
    (`PrimitiveComponent.SetCollisionEnabled` (`self.Cube3`) "NoCollision")
    (`PrimitiveComponent.SetCollisionEnabled` (`self.Cube4`) "NoCollision")
    (`PrimitiveComponent.SetCollisionEnabled` (`self.Cube5`) "NoCollision")
    (`PrimitiveComponent.SetCollisionEnabled` (`self.Cube6`) "NoCollision")
    (`KismetSystemLibrary.Delay` 1.0)
    (bind _returnvalue (`|CreateWidget` "/Game/Levels/Level_6/WB_Vita1.WB_Vita1_C"))
    (`UserWidget.AddToViewport` _returnvalue 0)
    (`KismetSystemLibrary.Delay` 4.0)
    (`WidgetLayoutLibrary.RemoveAllWidgets`)
    (bind _returnvalue_2 (`|CreateWidget` "/Game/Levels/Level_6/WB_Vita2.WB_Vita2_C"))
    (`UserWidget.AddToViewport` _returnvalue_2 0)
    (`KismetSystemLibrary.Delay` 2.0)
    (`WidgetLayoutLibrary.RemoveAllWidgets`)
    (bind _returnvalue_3 (`|CreateWidget` "/Game/Levels/Level_6/WB_Lena.WB_Lena_C"))
    (`UserWidget.AddToViewport` _returnvalue_3 0)
    (`KismetSystemLibrary.Delay` 5.0)
    (`WidgetLayoutLibrary.RemoveAllWidgets`)
    (`KismetSystemLibrary.QuitGame` null "Quit")))

(fn `UserConstructionScript`)