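; BP_Boss is a boss actor that takes damage whenever the player character overlaps its Box component.
; Each overlap lowers Health by one and prints a debug message.
; When Health reaches exactly zero, it finds the level's BP_Bridge through GetActorOfClass, calls BossDead on it and destroys itself.
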(event `self.Box.OnComponentBeginOverlap`
  (params (OverlappedComponent :type "PrimitiveComponent Object Reference") (OtherActor :type "Actor Object Reference") (OtherComp :type "PrimitiveComponent Object Reference") (OtherBodyIndex :type Integer) (bFromSweep :type Boolean) (SweepResult :type "HitResult Structure (by ref)"))
  (if (== OtherActor (`GameplayStatics.GetPlayerCharacter` 0))
    (set `self.Health` (- (`self.Health`) 1))
    (`KismetSystemLibrary.PrintString` "Damage")
    (if (== (`self.Health`) 0)
      (`KismetSystemLibrary.PrintString` "Boss Dead")
      (bind _returnvalue (`GameplayStatics.GetActorOfClass` "/Game/Actors/BP_Bridge.BP_Bridge_C"))
      (`/Game/Actors/BP_Bridge.BossDead` _returnvalue)
      (`self.K2_DestroyActor`))))

(fn `UserConstructionScript`)