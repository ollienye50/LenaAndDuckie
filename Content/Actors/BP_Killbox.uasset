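; BP_Killbox is a kill volume that sends the player back through the checkpoint system on contact.
; When the player pawn overlaps the Killbox component, it shows the WB_Death widget and calls Respawn on the level's BP_CheckpointTracker.
; After a short delay it clears every widget from the screen, not only the death widget.
; A disconnected branch that checks whether Level_6 is loaded never runs.
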(event `self.Killbox.OnComponentBeginOverlap`
  (params (OverlappedComponent :type "PrimitiveComponent Object Reference") (OtherActor :type "Actor Object Reference") (OtherComp :type "PrimitiveComponent Object Reference") (OtherBodyIndex :type Integer) (bFromSweep :type Boolean) (SweepResult :type "HitResult Structure (by ref)"))
  (if (== OtherActor (`GameplayStatics.GetPlayerPawn` 0))
    (`KismetSystemLibrary.PrintString` "duckie not dead")
    (bind _returnvalue (`|CreateWidget` "/Game/WB_Death.WB_Death_C"))
    (`UserWidget.AddToViewport` _returnvalue 0)
    (bind _returnvalue_2 (`GameplayStatics.GetActorOfClass` "/Game/Actors/BP_CheckpointTracker.BP_CheckpointTracker_C"))
    (`KismetSystemLibrary.PrintString` "Death")
    (`/Game/Actors/BP_CheckpointTracker.Respawn` _returnvalue_2)
    (`KismetSystemLibrary.Delay` 3.0)
    (`WidgetLayoutLibrary.RemoveAllWidgets`)))

(fn `UserConstructionScript`)