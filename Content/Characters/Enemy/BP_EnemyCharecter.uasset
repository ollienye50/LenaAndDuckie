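; BP_EnemyCharecter is a 2D side-view enemy character that follows the player's Lena character.
; From BeginPlay, FollowPlayer re-issues AI Move To every 0.2 seconds, targeting Lena, or itself when she is within 100 units.
; Tick sets control yaw to 0 or 180 from horizontal velocity to face the movement direction.
; UpdateAnimation is empty, and the idle/walk flipbook switch is disconnected.
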(event `self.ReceiveTick`
  (params (DeltaSeconds :type "Float (single-precision)"))
  (`self.UpdateAnimation`)
  (`self.UpdateControlRotation`))

(event `FollowPlayer`
  (if (>= (`self.GetDistanceTo` (`self.As BP Lena Character`)) 100.0)
    (`|AIMoveTo` self (0.0 0.0 0.0) (`self.As BP Lena Character`)
      (:`then`
        _))
    (else
      (`|AIMoveTo` self (0.0 0.0 0.0) self
        (:`then`
          _))))
  (`KismetSystemLibrary.Delay` 0.2)
  (`self.FollowPlayer`))

(event `self.ReceiveBeginPlay`
  (bind _asbp_lena_character (cast `/Game/Characters/Lena/BP_LenaCharacter` (`GameplayStatics.GetPlayerPawn` 0)))
  (set `self.As BP Lena Character` _asbp_lena_character)
  (`self.FollowPlayer`))

(event `UpdateControlRotation`
  (`/Engine/EditorBlueprintResources/StandardMacros.IsValid` (`self.GetController`)
    (:`Is Valid`
      (`/Engine/EditorBlueprintResources/StandardMacros.CompareFloat` (`KismetMathLibrary.BreakVector3f` (`MovementComponent.Velocity` (`self.CharacterMovement`)))
        (:`>`
          (`Controller.SetControlRotation` (`self.GetController`) (`KismetMathLibrary.MakeRotator` 0.0)))
        (:`<`
          (`Controller.SetControlRotation` (`self.GetController`) (`KismetMathLibrary.MakeRotator` 0.0 0.0 180.0)))))))

(fn `UpdateAnimation`)

(fn `UserConstructionScript`)