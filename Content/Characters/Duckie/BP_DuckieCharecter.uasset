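; BP_DuckieCharecter is a 2D flipbook character for Duckie that updates its animation and facing every tick.
; It picks the fall, walk or idle flipbook from the movement component's falling state and velocity.
; It turns by setting the controller's yaw to face along the sign of X velocity, keeping the last facing when X velocity is zero.
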(event `self.ReceiveTick`
  (params (DeltaSeconds :type "Float (single-precision)"))
  (`self.UpdateAnimation`)
  (`self.UpdateControlRotation`))

(event `UpdateAnimation`
  (`PaperFlipbookComponent.SetFlipbook` (`self.Sprite`) (select `bool` (`NavMovementComponent.IsFalling` (`self.CharacterMovement`)) :`false` (select `bool` (> (`KismetMathLibrary.VSize` (`MovementComponent.Velocity` (`self.CharacterMovement`))) 0.0) :`false` "/Game/Characters/Duckie/Animations/Idle/FB_DuckieIdle.FB_DuckieIdle" :`true` "/Game/Characters/Duckie/Animations/Walking/FB_DuckieWalk.FB_DuckieWalk" :!type "PaperFlipbook Object Reference") :`true` "/Game/Characters/Duckie/Animations/Falling/FB_DuckieFall.FB_DuckieFall")))

(event `UpdateControlRotation`
  (`/Engine/EditorBlueprintResources/StandardMacros.IsValid` (`self.GetController`)
    (:`Is Valid`
      (`/Engine/EditorBlueprintResources/StandardMacros.CompareFloat` (`KismetMathLibrary.BreakVector3f` (`MovementComponent.Velocity` (`self.CharacterMovement`)))
        (:`>`
          (`Controller.SetControlRotation` (`self.GetController`) (`KismetMathLibrary.MakeRotator` 0.0)))
        (:`<`
          (`Controller.SetControlRotation` (`self.GetController`) (`KismetMathLibrary.MakeRotator` 0.0 0.0 180.0)))))))

(fn `UserConstructionScript`)