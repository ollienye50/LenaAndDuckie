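; BP_Villager is a Level 4 villager that steps through a dialogue conversation in a WB_VillagerDialogue widget.
; Each VillagerDialogue call advances an index into the VDialogue lines, creating the widget if it is missing or otherwise updating its text.
; Index parity toggles the DuckieBase element, visible on even lines and hidden on odd ones, and the widget is removed once the lines run out.
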(event `/Game/Levels/Level_4/BPI_VillagerDialogue.VillagerDialogue`
  (`/Engine/EditorBlueprintResources/StandardMacros.IncrementInt` (`self.V_TalkIndex`)
    (:`  `
      (if (< (`self.V_TalkIndex`) (`KismetArrayLibrary.Array_Length` (`self.V_Dialogue`)))
        (`self.VillagerUI`
          (:`then`
            (`TextBlock.SetText` (`/Game/Levels/Level_4/WB_VillagerDialogue.VillagerText` (`self.VillagerUI`)) (`KismetTextLibrary.Conv_StringToText` (`|GetArrayItem` (`self.V_Dialogue`) (`self.V_TalkIndex`))))
            (if (> (mod (`self.V_TalkIndex`) 2) 0)
              (set `Widget.Visibility` "Hidden" (`/Game/Levels/Level_4/WB_VillagerDialogue.DuckieBase` (`self.VillagerUI`)))
              (else
                (set `Widget.Visibility` "Visible" (`/Game/Levels/Level_4/WB_VillagerDialogue.DuckieBase` (`self.VillagerUI`))))))
          (:`else`
            (bind _returnvalue (`|CreateWidget` "/Game/Levels/Level_4/WB_VillagerDialogue.WB_VillagerDialogue_C" (`GameplayStatics.GetPlayerController` 0)))
            (bind _output_get (set `self.VillagerUI` _returnvalue))
            (`UserWidget.AddToViewport` _output_get 0)))
        (else
          (`Widget.RemoveFromParent` (`self.VillagerUI`)))))))

(fn `UserConstructionScript`)